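; BP_Pawn is a player-controlled flying pawn that moves constantly forward, rolls, pitches, boosts and fires rockets.
; Tick feeds the forward vector into movement input, scaled by a boost value that rises while Boost is held.
; Roll and Pitch axes apply clamped, frame-rate-independent local rotations, and Fire spawns a short-lived BP_Rocket at the Arrow transform.
; BeginPlay registers the Right and Left components with BPSceneRotator.
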(event `self.ReceiveBeginPlay`
  (bind _scenecomponents (`/Game/BluePrints/BP_SceneRotator.SceneComponents` (`self.BP_SceneRotator`)))
  (`KismetArrayLibrary.Array_Add` _scenecomponents (`self.Right`))
  (`KismetArrayLibrary.Array_Add` _scenecomponents (`self.Left`)))

(event `InputAxis|Roll`
  (params (AxisValue :type "Float (single-precision)"))
  (`self.K2_AddActorLocalRotation` (`KismetMathLibrary.MakeRotator` (* (`KismetMathLibrary.FClamp` AxisValue -1.0) (`self.RotSpeed`) (`GameplayStatics.GetWorldDeltaSeconds`)))))

(event `InputAction|Boost`
  (params (Key :type "Key Structure"))
  (:`Pressed`
    (set `self.BoostScaleValue` 1.0))
  (:`Released`
    (set `self.BoostScaleValue` 0.5)))

(event `InputAction|Fire`
  (params (Key :type "Key Structure"))
  (:`Pressed`
    (bind _returnvalue (`|SpawnActorFromClass` "/Game/BluePrints/BP_Rocket.BP_Rocket_C" (`SceneComponent.K2_GetComponentToWorld` (`self.Arrow`)) "Undefined" "MultiplyWithRoot" self self))
    (`self.SetLifeSpan` _returnvalue 3.0)))

(event `InputAxis|Pitch`
  (params (AxisValue :type "Float (single-precision)"))
  (`self.K2_AddActorLocalRotation` (`KismetMathLibrary.MakeRotator` 0.0 (* (`KismetMathLibrary.FClamp` AxisValue -1.0) (`self.RotSpeed`) (`GameplayStatics.GetWorldDeltaSeconds`)))))

(event `self.ReceiveTick`
  (params (DeltaSeconds :type "Float (single-precision)"))
  (`self.AddMovementInput` (`self.GetActorForwardVector` self) (`self.BoostScaleValue`)))

(fn `UserConstructionScript`)